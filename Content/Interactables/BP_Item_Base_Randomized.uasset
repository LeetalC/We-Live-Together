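; Randomized item base Blueprint that varies the look of an interactable item when it is constructed.
; After the parent construction script, it assigns InteractableMesh a random static mesh from MeshArray.
; Optional RandomRotation and RandomSize flags add slight pitch and roll with free yaw, and a random non-uniform downscale.
; The randomization uses unseeded random calls, so results reroll whenever the construction script reruns.
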(fn `UserConstructionScript`
  (bind _returnvalue (`KismetMathLibrary.RandomFloatInRange` 0.3 0.7))
  (bind _returnvalue_2 (`KismetMathLibrary.RandomFloatInRange` -10.0 10.0))
  (bind _mesharray (`self.MeshArray`))
  (`parent.UserConstructionScript`)
  (`|ExecutionSequence`
    (:`then_0`
      (`StaticMeshComponent.SetStaticMesh` (`self.InteractableMesh`) (`|GetArrayItem` _mesharray (`KismetMathLibrary.RandomIntegerInRange` 0 (`KismetArrayLibrary.Array_LastIndex` _mesharray)))))
    (:`then_1`
      (if (`self.RandomRotation`)
        (`SceneComponent.K2_SetRelativeRotation` (`self.InteractableMesh`) (`KismetMathLibrary.MakeRotator` _returnvalue_2 _returnvalue_2 (`KismetMathLibrary.RandomFloatInRange` 0.0 360.0)) false false)))
    (:`then_2`
      (if (`self.RandomSize`)
        (`SceneComponent.SetRelativeScale3D` (`self.InteractableMesh`) (`KismetMathLibrary.MakeVector` _returnvalue _returnvalue _returnvalue))))))