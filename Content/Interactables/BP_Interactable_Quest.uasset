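; Quest pickup actor that shows quest information on the HUD when any actor overlaps it.
; On overlap it hides itself, adds a UMG_HUD_QuestPickup widget to the viewport and fills it with the name, description and objective from a hard-coded row of DT_QuestInfo.
; If the row is found, it hides the widget after a short delay and destroys itself.
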(event `self.ReceiveActorBeginOverlap`
  (params (OtherActor :type "Actor Object Reference"))
  (`|ExecutionSequence`
    (:`then_0`
      (`self.SetActorHiddenInGame` true))
    (:`then_1`
      (bind _returnvalue (`|CreateWidget` "/Game/UI/UMG_HUD_QuestPickup.UMG_HUD_QuestPickup_C"))
      (bind _output_get (set `self.HUDQuestPickup` _returnvalue))
      (`UserWidget.AddToViewport` _output_get 0))
    (:`then_2`
      (bind _returnvalue_2 (`|GetDataTableRow` "/Game/Quest/DT_QuestInfo.DT_QuestInfo" "1")
        (:`then`
          (`/Game/UI/UMG_HUD_QuestPickup.SetQuestDisplayText` (`self.HUDQuestPickup`) (break `/Game/Quest/F_QuestInfo` _returnvalue_2) (`.QuestDescription_7_790443CA4A15F448FFA5A2A7F159D89E` (break `/Game/Quest/F_QuestInfo` _returnvalue_2)) (`.QuestObjective_21_FAB5BAFE474D64AF3049DF9C990EEDED` (break `/Game/Quest/F_QuestInfo` _returnvalue_2)))
          (`KismetSystemLibrary.Delay` 5.0)
          (`Widget.SetVisibility` _returnvalue "Hidden")
          (`self.K2_DestroyActor`))))))

(fn `UserConstructionScript`
  (`parent.UserConstructionScript`))