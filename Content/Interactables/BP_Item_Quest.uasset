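; BP_Item_Quest is an interactable item that completes a quest when interacted with.
; Its construction script runs the parent's, then copies ThisQuestID into the QuestComponent.
; Quest activation switches on QuestParticles.
; Interaction completes the quest and runs the parent interaction only if the quest is both activated and unlocked; otherwise it does nothing.
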(event `self.Interaction`
  (params (Instigator :type "/Game/Blueprints/BP_RPGCharacter Object Reference"))
  (bind _questcomponent (`self.QuestComponent`))
  (if (and (`/Game/Quest/QuestComponent.IsQuestActivated` _questcomponent) (`/Game/Quest/QuestComponent.IsQuestUnlocked` _questcomponent))
    (`/Game/Quest/QuestComponent.CompleteQuest` (`self.QuestComponent`))
    (`parent.Interaction` Instigator)))

(event `self.QuestComponent.QuestActivated`
  (`ActorComponent.SetActive` (`self.QuestParticles`) true false))

(fn `UserConstructionScript`
  (`parent.UserConstructionScript`)
  (set `/Game/Quest/QuestComponent.QuestID` (`self.ThisQuestID`) (`self.QuestComponent`)))