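; Quest interactable for a baby deer that starts hidden, shows particles when its quest activates, and can move along a spline path.
; MoveBabyDeer drives location and rotation along the path spline with a timeline scaled to a set duration.
; Interaction fades a black screen, teleports the player, completes the quest and signals that the deer was found.
; It then spawns a BP_BabyDeer at a new transform and destroys the path and itself.
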(event `self.ReceiveBeginPlay`
  (`|ExecutionSequence`
    (:`then_0`
      (bind _asbp_rpgcharacter (cast `/Game/Blueprints/BP_RPGCharacter` (`GameplayStatics.GetPlayerCharacter` 0)))
      (set `self.Character` _asbp_rpgcharacter))
    (:`then_1`
      (`self.SetActorHiddenInGame` true)
      (`SceneComponent.SetVisibility` (`self.QuestParticles`) false false))))

(event `MoveBabyDeer`
  (bind _pathspline (`/Game/Blueprints/BP_BabyDeerPath.PathSpline` (`self.Path`)))
  (`TimelineComponent.SetPlayRate` (`self.BabyDeerMover_Timeline`) (/ 1.0 (`self.Duration`)))
  (bind (_direction _alpha) (`Timeline|BabyDeerMover_Timeline`)
    (:`Update`
      (bind _returnvalue (`KismetMathLibrary.Lerp` 0.0 (`SplineComponent.GetSplineLength` _pathspline) _alpha))
      (`self.K2_SetActorLocationAndRotation` (`SplineComponent.GetLocationAtDistanceAlongSpline` _pathspline _returnvalue "World") (`SplineComponent.GetRotationAtDistanceAlongSpline` _pathspline _returnvalue "Local")))))

(event `self.QuestComponent.QuestActivated`
  (`SceneComponent.SetVisibility` (`self.QuestParticles`) true false))

(event `/Game/Interactables/BPI_Interactor.Interaction`
  (params (Instigator :type "/Game/Blueprints/BP_RPGCharacter Object Reference"))
  (bind _returnvalue (`|CreateWidget` "/Game/UI/UMG_BlackScreen.UMG_BlackScreen_C"))
  (`/Game/UI/UMG_BlackScreen.FullFade` _returnvalue)
  (`UserWidget.AddToViewport` _returnvalue 0)
  (set `self.ActivelyRunning` false)
  (`KismetSystemLibrary.Delay` 2.0)
  (`|ExecutionSequence`
    (:`then_0`
      (`self.K2_SetActorLocation` (`self.Character`) (`self.TeleportLocation`) false true))
    (:`then_1`
      (`KismetSystemLibrary.Delay` 1.0)
      (`/Game/Quest/QuestComponent.CompleteQuest` (`self.QuestComponent`))
      (`self.BabyDeerFoundWasCompleted`)
      (`|SpawnActorFromClass` "/Game/Blueprints/BP_BabyDeer.BP_BabyDeer_C" (`self.NewLocForBabyDeer`) "Undefined" "OverrideRootScale" null null)
      (`self.K2_DestroyActor` (`self.Path`))
      (`self.K2_DestroyActor`))))

(fn `UserConstructionScript`
  (`parent.UserConstructionScript`))