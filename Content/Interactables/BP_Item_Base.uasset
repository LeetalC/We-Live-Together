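; Base interactable item that hands its info to whoever interacts with it.
; Construction fills ItemInfo from the DT_ItemInfo row named by RowName, adding the actor's own class.
; It also randomizes the mesh from MeshArray, its scale independently per axis, and optionally its rotation.
; Interaction calls PickUp on the instigator, with an eating sound and actor destruction each set behind a short delay.
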(event `/Game/Interactables/BPI_Interactor.Interaction`
  (params (Instigator :type "/Game/Blueprints/BP_RPGCharacter Object Reference"))
  (`|ExecutionSequence`
    (:`then_0`
      (`KismetSystemLibrary.Delay` 0.5)
      (`GameplayStatics.PlaySoundAtLocation` (`self.EatingSound`) (`self.K2_GetActorLocation`) (struct) 1.0 1.0 0.0 null null null))
    (:`then_1`
      (`/Game/Interactables/BPI_Interactor.PickUp` Instigator (`self.ItemInfo`))
      (`KismetSystemLibrary.Delay` 0.5)
      (`self.K2_DestroyActor`))))

(fn `UserConstructionScript`
  (bind _returnvalue (`KismetMathLibrary.RandomFloatInRange` 0.5 0.9))
  (bind _returnvalue_2 (`KismetMathLibrary.RandomFloatInRange` -10.0 10.0))
  (bind _mesharray (`self.MeshArray`))
  (`parent.UserConstructionScript`)
  (`|ExecutionSequence`
    (:`then_0`
      (bind _returnvalue_3 (`|GetDataTableRow` "/Game/Interactables/DT_ItemInfo.DT_ItemInfo" (`self.RowName`))
        (:`then`
          (set `self.ItemInfo` (make `/Game/Interactables/F_ItemInfo` (break `/Game/Interactables/F_ItemInfo` _returnvalue_3) (`.ItemImg_20_D218C0EF482E3DF243E259AF5FE6A772` (break `/Game/Interactables/F_ItemInfo` _returnvalue_3)) (`GameplayStatics.GetObjectClass` self) (`.ItemDescrip_29_E8BCDBA247D99FBFD42BE6B1E8EAEE78` (break `/Game/Interactables/F_ItemInfo` _returnvalue_3)) (`.ItemType_39_2F5179FD460A991453667BB27B3F6859` (break `/Game/Interactables/F_ItemInfo` _returnvalue_3)) (`.StaminaValue_35_48BB34704AA0F5CAA4967CBD3FA327B6` (break `/Game/Interactables/F_ItemInfo` _returnvalue_3)) (`.HappinessValue_40_757AC70248A34FA56B2C968AA20E90F9` (break `/Game/Interactables/F_ItemInfo` _returnvalue_3)))))))
    (:`then_1`
      (`StaticMeshComponent.SetStaticMesh` (`self.InteractableMesh`) (`|GetArrayItem` _mesharray (`KismetMathLibrary.RandomIntegerInRange` 0 (`KismetArrayLibrary.Array_LastIndex` _mesharray)))))
    (:`then_2`
      (if (`self.RandomRotation`)
        (`SceneComponent.K2_SetRelativeRotation` (`self.InteractableMesh`) (`KismetMathLibrary.MakeRotator` _returnvalue_2 _returnvalue_2 (`KismetMathLibrary.RandomFloatInRange` 0.0 360.0)) false false)))
    (:`then_3`
      (`SceneComponent.SetRelativeScale3D` (`self.InteractableMesh`) (`KismetMathLibrary.MakeVector` _returnvalue _returnvalue _returnvalue)))))