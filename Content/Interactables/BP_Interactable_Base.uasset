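; Base interactable Blueprint that lets the RPG character detect nearby objects and receive feedback on them.
; A sphere collider, sized from InteractableRadius in the Construction Script, registers and unregisters the object with any overlapping BP_RPGCharacter.
; BeginPlay caches the mesh's default material and the player character.
; SetFeedback toggles the interaction particles, while InventoryFeedback prints an on-screen item pickup message.
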(event `self.ReceiveBeginPlay`
  (`|ExecutionSequence`
    (:`then_0`
      (set `self.DefaultMaterial` (`PrimitiveComponent.GetMaterial` (`self.InteractableMesh`) 0)))
    (:`then_1`
      (bind _asbp_rpgcharacter (cast `/Game/Blueprints/BP_RPGCharacter` (`GameplayStatics.GetPlayerCharacter` 0)))
      (set `self.Character` _asbp_rpgcharacter))))

(event `self.InteractableCollider.OnComponentBeginOverlap`
  (params (OverlappedComponent :type "PrimitiveComponent Object Reference") (OtherActor :type "Actor Object Reference") (OtherComp :type "PrimitiveComponent Object Reference") (OtherBodyIndex :type Integer) (bFromSweep :type Boolean) (SweepResult :type "HitResult Structure (by ref)"))
  (bind _asbp_rpgcharacter (cast `/Game/Blueprints/BP_RPGCharacter` OtherActor))
  (message `/Game/Interactables/BPI_Interactor.RegisterInteractable` _asbp_rpgcharacter self))

(event `self.InteractableCollider.OnComponentEndOverlap`
  (params (OverlappedComponent :type "PrimitiveComponent Object Reference") (OtherActor :type "Actor Object Reference") (OtherComp :type "PrimitiveComponent Object Reference") (OtherBodyIndex :type Integer))
  (bind _asbp_rpgcharacter (cast `/Game/Blueprints/BP_RPGCharacter` OtherActor))
  (message `/Game/Interactables/BPI_Interactor.UnregisterInteractable` _asbp_rpgcharacter self))

(fn `InventoryFeedback`
  (params (ItemInfo :type "/Game/Interactables/F_ItemInfo Structure"))
  (`KismetSystemLibrary.PrintText` (`KismetTextLibrary.Conv_StringToText` (`KismetStringLibrary.Concat_StrStr` (`KismetTextLibrary.Conv_TextToString` ItemInfo_ItemName_19_8E0F696F42F41366546F298C210EBD48) " was picked up.")) true true (struct :`G` 1.0 :`B` 0.180493 :`A` 1.0) 15.0))

(fn `SetFeedback`
  (params (`Give Feedback` :type Boolean))
  (`ActorComponent.SetActive` (`self.InteractionParticles`) `Give Feedback` false))

(fn `UserConstructionScript`
  (`SphereComponent.SetSphereRadius` (`self.InteractableCollider`) (`self.InteractableRadius`) true))