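; BP_QuestTrigger_Activator is a world trigger that activates a quest when its collider is overlapped while that quest is unlocked.
; The QuestComponent unlock event turns on the quest marker particles, and an overlap plays a notification sound and calls ActivateQuest.
; On activation, the actor hides the marker, disables collision and destroys itself after a short delay.
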(event `self.Collider.OnComponentBeginOverlap`
  (params (OverlappedComponent :type "PrimitiveComponent Object Reference") (OtherActor :type "Actor Object Reference") (OtherComp :type "PrimitiveComponent Object Reference") (OtherBodyIndex :type Integer) (bFromSweep :type Boolean) (SweepResult :type "HitResult Structure (by ref)"))
  (if (`/Game/Quest/QuestComponent.IsQuestUnlocked` (`self.QuestComponent`))
    (`GameplayStatics.PlaySound2D` "/Game/SoundFX/SFX/Notification_Quest.Notification_Quest" 0.5 0.8 0.0 null null)
    (`/Game/Quest/QuestComponent.ActivateQuest` (`self.QuestComponent`))))

(event `self.QuestComponent.QuestUnlocked`
  (`ActorComponent.SetActive` (`self.QuestMarkerParticles`) true false))

(event `self.QuestComponent.QuestActivated`
  (`ActorComponent.SetActive` (`self.QuestMarkerParticles`) false false)
  (`PrimitiveComponent.SetCollisionEnabled` (`self.Collider`) "NoCollision")
  (`KismetSystemLibrary.Delay` 5.0)
  (`self.K2_DestroyActor`))

(fn `UserConstructionScript`
  (`parent.UserConstructionScript`))