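; Quest trigger actor that completes its quest when something overlaps its collider.
; The overlap only counts while the QuestComponent is both activated and unlocked, then plays a notification sound and calls CompleteQuest.
; Component events drive the marker particles, turning them on at activation and off at completion.
; Completion also disables the collider and destroys the actor after a short delay.
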(event `self.Collider.OnComponentBeginOverlap`
  (params (OverlappedComponent :type "PrimitiveComponent Object Reference") (OtherActor :type "Actor Object Reference") (OtherComp :type "PrimitiveComponent Object Reference") (OtherBodyIndex :type Integer) (bFromSweep :type Boolean) (SweepResult :type "HitResult Structure (by ref)"))
  (bind _questcomponent (`self.QuestComponent`))
  (if (and (`/Game/Quest/QuestComponent.IsQuestActivated` _questcomponent) (`/Game/Quest/QuestComponent.IsQuestUnlocked` _questcomponent))
    (`GameplayStatics.PlaySound2D` "/Game/SoundFX/SFX/Notification_Quest1.Notification_Quest1" 0.5 1.1 0.0 null null)
    (`/Game/Quest/QuestComponent.CompleteQuest` (`self.QuestComponent`))))

(event `self.QuestComponent.QuestActivated`
  (`ActorComponent.SetActive` (`self.QuestMarkerParticles`) true false))

(event `self.QuestComponent.QuestCompleted`
  (`ActorComponent.SetActive` (`self.QuestMarkerParticles`) false false)
  (`PrimitiveComponent.SetCollisionEnabled` (`self.Collider`) "NoCollision")
  (`KismetSystemLibrary.Delay` 5.0)
  (`self.K2_DestroyActor`))

(fn `UserConstructionScript`
  (`parent.UserConstructionScript`))