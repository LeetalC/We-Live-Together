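; BP_Quest is a quest pickup actor that gives the player its quest when its collider is overlapped.
; Overlap turns off the marker particles, notifies the RPG character of the active quest and shows a timed HUD popup before destroying itself.
; AddToQuestLog appends the quest info to the character's log and adds a matching log widget.
; Game instance quest events are bound to debug prints with mismatched labels.
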(event `self.ReceiveBeginPlay`
  (`|ExecutionSequence`
    (:`then_0`
      (bind _asbp_rpgcharacter (cast `/Game/Blueprints/BP_RPGCharacter` (`GameplayStatics.GetPlayerCharacter` 0)))
      (set `self.Character` _asbp_rpgcharacter))
    (:`then_1`
      (bind _asbp_rpggame_instance (cast `/Game/Blueprints/BP_RPGGameInstance` (`GameplayStatics.GetGameInstance`)))
      (`|ExecutionSequence`
        (:`then_0`
          (add `/Game/Blueprints/BP_RPGGameInstance.QuestActivated` _asbp_rpggame_instance (delegate `QuestActivated`)))
        (:`then_1`
          (add `/Game/Blueprints/BP_RPGGameInstance.QuestCompleted` _asbp_rpggame_instance (delegate `QuestCompleted`)))
        (:`then_2`
          (add `/Game/Blueprints/BP_RPGGameInstance.QuestUnlocked` _asbp_rpggame_instance (delegate `QuestUnlocked`)))))))

(event `QuestActivated`
  (params (ID :type "GameplayTag Structure (by ref)"))
  (`KismetSystemLibrary.PrintString` (`KismetStringLibrary.Concat_StrStr` "BP Completed " (`KismetStringLibrary.Conv_NameToString` (`BlueprintGameplayTagLibrary.GetTagName` ID)))))

(event `QuestCompleted`
  (params (ID :type "GameplayTag Structure (by ref)"))
  (`KismetSystemLibrary.PrintString` (`KismetStringLibrary.Concat_StrStr` "BP Unlocked " (`KismetStringLibrary.Conv_NameToString` (`BlueprintGameplayTagLibrary.GetTagName` ID)))))

(event `QuestUnlocked`
  (params (ID :type "GameplayTag Structure (by ref)"))
  (`KismetSystemLibrary.PrintString` (`KismetStringLibrary.Concat_StrStr` "BP Activated " (`KismetStringLibrary.Conv_NameToString` (`BlueprintGameplayTagLibrary.GetTagName` ID)))))

(event `self.Collider.OnComponentBeginOverlap`
  (params (OverlappedComponent :type "PrimitiveComponent Object Reference") (OtherActor :type "Actor Object Reference") (OtherComp :type "PrimitiveComponent Object Reference") (OtherBodyIndex :type Integer) (bFromSweep :type Boolean) (SweepResult :type "HitResult Structure (by ref)"))
  (bind (_thisquestinfo_id _thisquestinfo_startsquestline _thisquestinfo_questname _thisquestinfo_questdescription _thisquestinfo_questobjective) (break `/Game/Quest/F_QuestInfo` (`self.ThisQuestInfo`)))
  (`|ExecutionSequence`
    (:`then_0`
      (`ActorComponent.SetActive` (`self.QuestMarkerParticles`) false false)
      (`/Game/Blueprints/BP_RPGCharacter.Active Quest Changed` (`self.Character`) (`self.ThisQuestRowName`)))
    (:`then_1`
      (bind _returnvalue (`|CreateWidget` "/Game/UI/UMG_HUD_QuestPickup.UMG_HUD_QuestPickup_C"))
      (bind _output_get (set `self.HUDQuest Pickup` _returnvalue))
      (`UserWidget.AddToViewport` _output_get 0))
    (:`then_2`
      (`/Game/UI/UMG_HUD_QuestPickup.SetQuestDisplayText` (`self.HUDQuest Pickup`) _thisquestinfo_questname _thisquestinfo_questdescription _thisquestinfo_questobjective)
      (`self.AddToQuestLog`)
      (`KismetSystemLibrary.Delay` (`self.QuestPickupOnScreenTime`))
      (`Widget.RemoveFromParent` _returnvalue)
      (`self.K2_DestroyActor`))))

(fn `AddToQuestLog`
  (bind (_id _startsquestline _questname _questdescription _questobjective _questreward _isunlocked _iscomplete _isactive _automaticallycontinuetonextquest _manualqueststounlock) (break `/Game/Quest/F_QuestInfo` (`self.ThisQuestInfo`)))
  (`KismetArrayLibrary.Array_Add` (`/Game/Blueprints/BP_RPGCharacter.QuestLog` (`self.Character`)) (make `/Game/Quest/F_QuestInfo` (struct) false _questname _questdescription _questobjective _questreward false false false false _manualqueststounlock))
  (bind _returnvalue (`|CreateWidget` "/Game/UI/UMG_QuestLog_QuestInfo.UMG_QuestLog_QuestInfo_C"))
  (bind _output_get (set `self.UMGQuestLog_QuestInfo` _returnvalue))
  (`/Game/UI/UMG_QuestLog_QuestInfo.SetQuestInfosText` _output_get _questname _questdescription _questobjective (`KismetTextLibrary.Conv_IntToText` _questreward))
  (`/Game/UI/UMG_QuestLog.AddQuest` (`/Game/Blueprints/BP_RPGCharacter.UMGQuestLog` (`self.Character`)) _returnvalue))

(fn `UserConstructionScript`)