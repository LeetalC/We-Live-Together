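; Quest completion trigger for the water bucket quest, staging the scene in which water is delivered to the doe.
; On QuestCompleted it freezes the player's movement, runs a full black-screen fade and, after a delay, moves the player's bucket onto the quest marker mesh.
; After a further delay it rotates and animates the stag and doe, restores walking and calls WaterForDoeWasCompleted.
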(event `self.ReceiveBeginPlay`
  (bind _asbp_rpgcharacter (cast `/Game/Blueprints/BP_RPGCharacter` (`GameplayStatics.GetPlayerCharacter` 0)))
  (set `self.Character` _asbp_rpgcharacter))

(event `self.QuestComponent.QuestCompleted`
  (bind _momdoemesh (`/Game/Blueprints/BP_MomDoe.MomDoeMesh` (`self.MomDoe`)))
  (bind _dadstagmesh (`/Game/Blueprints/BP_Stag.DadStagMesh` (`self.DadStag`)))
  (`CharacterMovementComponent.SetMovementMode` (`Character.CharacterMovement` (`self.Character`)) "MOVE_None" 0)
  (bind _returnvalue (`|CreateWidget` "/Game/UI/UMG_BlackScreen.UMG_BlackScreen_C"))
  (`/Game/UI/UMG_BlackScreen.FullFade` _returnvalue)
  (`UserWidget.AddToViewport` _returnvalue 0)
  (`KismetSystemLibrary.Delay` 1.0)
  (`/Game/Quest/BP_Bucket.AttachBucketToComponent` (`/Game/Blueprints/BP_RPGCharacter.Bucket` (`self.Character`)) (`self.QuestMarkerMesh`))
  (`KismetSystemLibrary.Delay` 3.0)
  (`SceneComponent.K2_AddLocalRotation` _dadstagmesh (struct :`Yaw` 30.0) false false)
  (`SkeletalMeshComponent.PlayAnimation` _dadstagmesh "/Game/ContentPacks/AnimalVarietyPack/DeerStagAndDoe/Animations/ANIM_DeerStag_IdleBreathe.ANIM_DeerStag_IdleBreathe" false)
  (`SceneComponent.K2_AddLocalRotation` _momdoemesh (struct :`Yaw` 50.0) false false)
  (`SkeletalMeshComponent.PlayAnimation` _momdoemesh "/Game/ContentPacks/AnimalVarietyPack/DeerStagAndDoe/Animations/ANIM_DeerDoe_RestToGoBackUp.ANIM_DeerDoe_RestToGoBackUp" false)
  (`CharacterMovementComponent.SetMovementMode` (`Character.CharacterMovement` (`self.Character`)) "MOVE_Walking" 0)
  (`self.WaterForDoeWasCompleted`))

(fn `UserConstructionScript`
  (`parent.UserConstructionScript`))