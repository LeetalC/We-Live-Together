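; Quest trigger for the stag quest skip that unlocks the player's Dash and reveals the baby deer.
; Unlocking the quest turns on marker particles; an overlap while unlocked plays a sound, activates the quest, unlocks Dash, then shows and moves the deer.
; Activation hides the marker, disables the collider and immediately completes the quest.
; Completion destroys the actor after a short delay.
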(event `self.ReceiveBeginPlay`
  (bind _asbp_rpgcharacter (cast `/Game/Blueprints/BP_RPGCharacter` (`GameplayStatics.GetPlayerCharacter` 0)))
  (set `self.Character` _asbp_rpgcharacter))

(event `self.Collider.OnComponentBeginOverlap`
  (params (OverlappedComponent :type "PrimitiveComponent Object Reference") (OtherActor :type "Actor Object Reference") (OtherComp :type "PrimitiveComponent Object Reference") (OtherBodyIndex :type Integer) (bFromSweep :type Boolean) (SweepResult :type "HitResult Structure (by ref)"))
  (bind _babydeer (`self.BabyDeer`))
  (if (`/Game/Quest/QuestComponent.IsQuestUnlocked` (`self.QuestComponent`))
    (`GameplayStatics.PlaySound2D` "/Game/SoundFX/SFX/Notification_Quest.Notification_Quest" 0.5 0.8 0.0 null null)
    (`/Game/Quest/QuestComponent.ActivateQuest` (`self.QuestComponent`))
    (set `/Game/Blueprints/AbilitiesComponent.DashUnlocked` true (`/Game/Blueprints/BP_RPGCharacter.AbilitiesComponent` (`self.Character`)))
    (`self.SetActorHiddenInGame` _babydeer false)
    (`/Game/Interactables/BP_Item_Quest_BabyDeer.MoveBabyDeer` _babydeer)))

(event `self.QuestComponent.QuestUnlocked`
  (`ActorComponent.SetActive` (`self.QuestMarkerParticles`) true false))

(event `self.QuestComponent.QuestActivated`
  (`ActorComponent.SetActive` (`self.QuestMarkerParticles`) false false)
  (`PrimitiveComponent.SetCollisionEnabled` (`self.Collider`) "NoCollision")
  (`/Game/Quest/QuestComponent.CompleteQuest` (`self.QuestComponent`)))

(event `self.QuestComponent.QuestCompleted`
  (`KismetSystemLibrary.Delay` 1.0)
  (`self.K2_DestroyActor`))

(fn `UserConstructionScript`
  (`parent.UserConstructionScript`))