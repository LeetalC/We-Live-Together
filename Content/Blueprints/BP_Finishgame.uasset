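; BP_Finishgame is an actor that ends the game once both the mom and baby deer quests are complete.
; On BeginPlay it caches the player RPG character and binds to completion events on the two quest triggers, each setting a flag and rechecking both.
; When both flags are set, it waits briefly, then shows the demo screen through the character's HUD widget with cursor capture.
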(event `self.ReceiveBeginPlay`
  (bind _asbp_rpgcharacter (cast `/Game/Blueprints/BP_RPGCharacter` (`GameplayStatics.GetPlayerCharacter` 0)))
  (set `self.Character` _asbp_rpgcharacter)
  (add `/Game/Quest/BP_QuestTrigger_Completor_Bucket.WaterForDoeWasCompleted` (`self.QuestMomTrigger`) (delegate `MomQuestFinished`))
  (add `/Game/Interactables/BP_Item_Quest_BabyDeer.BabyDeerFoundWasCompleted` (`self.QuestBabyTrigger`) (delegate `BabyQuestFinished`)))

(event `MomQuestFinished`
  (set `self.QuestMomComplete` true)
  (`self.CheckForFinishGame` :!label _label))

(event `BabyQuestFinished`
  (set `self.QuestBabyComplete` true)
  (goto _label))

(event `CheckForFinishGame`
  (if (and (`self.QuestBabyComplete`) (`self.QuestMomComplete`))
    (`self.FinishGame`)))

(event `FinishGame`
  (bind _hudwidget (`/Game/Blueprints/BP_RPGCharacter.HUDWidget` (`self.Character`)))
  (`KismetSystemLibrary.Delay` 5.0)
  (`/Game/UI/UMG_MainHUD.ActivateNotificationWidget` _hudwidget (`/Game/UI/UMG_MainHUD.UMG_DemoScreen` _hudwidget) true true false))

(fn `UserConstructionScript`)