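; RPG game mode that manages 2D background music.
; On BeginPlay it spawns the BGMusic track at a lowered pitch, fades it in and keeps it in TempSound.
; The MusicChanged event fades out and stops that sound after a delay, then spawns BGMusic again at normal pitch with a fade-in.
; An Acid Rain ambient loop branch is present but disconnected.
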(event `MusicChanged`
  (bind _tempsound (`self.TempSound`))
  (bind _musicfadetime (`self.MusicFadeTime`))
  (`AudioComponent.FadeOut` _tempsound _musicfadetime 0.0)
  (`KismetSystemLibrary.Delay` (+ _musicfadetime 1.0))
  (`AudioComponent.Stop` _tempsound)
  (bind _returnvalue (`GameplayStatics.SpawnSound2D` (`self.BGMusic`) 0.7 1.0 0.0 null))
  (`AudioComponent.FadeIn` _returnvalue 2.0 1.0 0.0)
  (set `self.TempSound` _returnvalue))

(event `self.ReceiveBeginPlay`
  (bind _returnvalue (`GameplayStatics.SpawnSound2D` (`self.BGMusic`) 0.8 0.7 0.0 null))
  (`AudioComponent.FadeIn` _returnvalue 5.0 1.0 0.0)
  (set `self.TempSound` _returnvalue))

(fn `UserConstructionScript`)