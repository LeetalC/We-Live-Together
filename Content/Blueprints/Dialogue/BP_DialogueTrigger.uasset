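; BP_DialogueTrigger is a one-shot trigger that plays a line of dialogue on the player's HUD when its collider is overlapped.
; BeginPlay caches the player as BP_RPGCharacter.
; Any overlap, with no check on the overlapping actor, looks up RowNameDialogue in DT_Dialogue.
; If the row is found, its text goes to the HUD's UMGDialogue PlayDialogue and the trigger destroys itself.
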(event `self.ReceiveBeginPlay`
  (bind _asbp_rpgcharacter (cast `/Game/Blueprints/BP_RPGCharacter` (`GameplayStatics.GetPlayerCharacter` 0)))
  (set `self.Character` _asbp_rpgcharacter))

(event `self.TriggerDialogueCollider.OnComponentBeginOverlap`
  (params (OverlappedComponent :type "PrimitiveComponent Object Reference") (OtherActor :type "Actor Object Reference") (OtherComp :type "PrimitiveComponent Object Reference") (OtherBodyIndex :type Integer) (bFromSweep :type Boolean) (SweepResult :type "HitResult Structure (by ref)"))
  (bind _returnvalue (`|GetDataTableRow` "/Game/Blueprints/Dialogue/DT_Dialogue.DT_Dialogue" (`self.RowName_Dialogue`))
    (:`then`
      (`/Game/UI/Notifications/UMG_Dialogue.PlayDialogue` (`/Game/UI/UMG_MainHUD.UMG_Dialogue` (`/Game/Blueprints/BP_RPGCharacter.HUDWidget` (`self.Character`))) (`.Text_5_6707EE2D43BB85E5B6CF51A2EE4CAEEE` (break `/Game/Blueprints/Dialogue/F_Dialogue` _returnvalue)))
      (`self.K2_DestroyActor`))))

(fn `UserConstructionScript`)