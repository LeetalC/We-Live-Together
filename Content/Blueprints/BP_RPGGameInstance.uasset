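; Game instance that acts as the RPG's central quest manager, tracking each quest's unlocked, active and completed state.
; On Init it loads DT_QuestInfo into a map keyed by gameplay tag.
; Unlock, Activate and Complete events write updated structs back into the map, maintain the active quest list and notify listeners.
; Completion unlocks either the next quest in key order or a manual list, and unlocking can auto-activate.
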(event `self.ReceiveInit`
  (`|ExecutionSequence`
    (:`then_0`
      (bind _outrownames (`DataTableFunctionLibrary.GetDataTableRowNames` "/Game/Quest/DT_QuestInfo.DT_QuestInfo"))
      (for _array_element _outrownames
        (bind _returnvalue (`|GetDataTableRow` "/Game/Quest/DT_QuestInfo.DT_QuestInfo" _array_element)
          (:`then`
            (`BlueprintMapLibrary.Map_Add` (`self.QuestDatabase`) (`.ID_39_5D90E7484066EB3FB036638B1FDA7246` (break `/Game/Quest/F_QuestInfo` _returnvalue)) _returnvalue) ; Using a map. ID = keys, FQuestInfo = values. The IDs are gameplay tag.
          ))))))

(event `CompleteQuestWithID`
  (params (ID :type "GameplayTag Structure (by ref)"))
  (bind _currentid (`self.CurrentID`))
  (bind _activequests (`self.ActiveQuests`))
  (bind (_value _returnvalue) (`BlueprintMapLibrary.Map_Find` (`self.QuestDatabase`) ID))
  (bind ((`AutomaticallyUnlockNextQuest_58_A47F517B44C9DFBDD149B899E73F4504` _automaticallyunlocknextquest) (`ManualQuestsToUnlock_53_9A993881425B5300D5456A8F9210F98A` _manualqueststounlock)) (break `/Game/Quest/F_QuestInfo` _value))
  (set `self.CurrentID` ID)
  (if _returnvalue
    (bind _structout (setmembers `/Game/Quest/F_QuestInfo` :`StructRef` _value :`IsComplete` true)) ; Mark the quest complete. (The current quest, \nnot the one that is immediatly assigned afterwards)
    (`BlueprintMapLibrary.Map_Add` (`self.QuestDatabase`) (`self.CurrentID`) _structout) ; Overwriting the current quest
    (`KismetArrayLibrary.Array_RemoveItem` _activequests (`self.CurrentID`)) ; Removing the quest from ActiveQuests
    (set `self.IsPlayerInQuest` (> (`KismetArrayLibrary.Array_Length` _activequests) 0)) ; So far not using this, but checking \nif the player is on any quest
    (`|ExecutionSequence`
      (:`then_0`
        (`self.QuestCompletedWithID` _currentid) ; Tell everything listening  that the quest is complete
        (`KismetSystemLibrary.PrintString` (`KismetStringLibrary.Concat_StrStr` (`KismetStringLibrary.Conv_NameToString` (`BlueprintGameplayTagLibrary.GetTagName` _currentid)) " was just completed from GAMEINSTANCE") true true (struct :`G` 1.0 :`B` 0.011483 :`A` 1.0) 5.0))
      (:`then_1`
        (if _automaticallyunlocknextquest
          (bind _keys (`BlueprintMapLibrary.Map_Keys` (`self.QuestDatabase`)))
          (bind _result (`/Engine/EditorBlueprintResources/StandardMacros.IncrementInt` (`KismetArrayLibrary.Array_Find` _keys (`self.CurrentID`)))
            (:`  `
              (bind _output (`|GetArrayItem` _keys _result))
              (`self.UnlockQuestWithID` _output) ; This is supposed to iterate to the next quest if the previous quest was \nmarked as 'Automatically continue to the next quest'\nPlaces where this is used:\nIf the next quest is an 'objective'
              (`KismetSystemLibrary.PrintString` (`KismetStringLibrary.Concat_StrStr` "Automatically Unlocking this quest: " (`KismetStringLibrary.Conv_NameToString` (`BlueprintGameplayTagLibrary.GetTagName` _output))) true true (struct :`R` 1.0 :`G` 0.126577 :`A` 1.0) 5.0)))
          (elif (> (`KismetArrayLibrary.Array_Length` _manualqueststounlock) 0)
            (for _array_element _manualqueststounlock
              (`self.UnlockQuestWithID` _array_element) ; Unlock them individually
              (`KismetSystemLibrary.PrintString` (`KismetStringLibrary.Concat_StrStr` "Manually Unlocking this quest: " (`KismetStringLibrary.Conv_NameToString` (`BlueprintGameplayTagLibrary.GetTagName` _array_element))) true true (struct :`R` 1.0 :`G` 0.529868 :`A` 1.0) 5.0))))))
    (else
      (`KismetSystemLibrary.PrintString` (`KismetStringLibrary.Concat_StrStr` "Could not complete quest with ID: " (`KismetStringLibrary.Conv_NameToString` (`BlueprintGameplayTagLibrary.GetTagName` ID)))))))

(event `UnlockQuestWithID`
  (params (ID :type "GameplayTag Structure (by ref)"))
  (bind _currentid (`self.CurrentID`))
  (bind (_value _returnvalue) (`BlueprintMapLibrary.Map_Find` (`self.QuestDatabase`) ID))
  (set `self.CurrentID` ID)
  (if _returnvalue
    (bind _structout (setmembers `/Game/Quest/F_QuestInfo` :`StructRef` _value :`IsUnlocked` true))
    (`BlueprintMapLibrary.Map_Add` (`self.QuestDatabase`) _currentid _structout)
    (`self.QuestUnlockedWithID` _currentid)
    (if (`.AutomaticallyActivateThisQuest_60_E1E433F44EAE5A5AD7B062B0D3DBB220` (break `/Game/Quest/F_QuestInfo` _value))
      (`self.ActivateQuestWithID` (`self.CurrentID`)))
    (else
      (`KismetSystemLibrary.PrintString` (`KismetStringLibrary.Concat_StrStr` "Could not unlock quest with ID: " (`KismetStringLibrary.Conv_NameToString` (`BlueprintGameplayTagLibrary.GetTagName` ID)))))))

(event `ActivateQuestWithID`
  (params (ID :type "GameplayTag Structure (by ref)"))
  (bind _currentid (`self.CurrentID`))
  (bind (_value _returnvalue) (`BlueprintMapLibrary.Map_Find` (`self.QuestDatabase`) ID))
  (set `self.CurrentID` ID)
  (if _returnvalue
    (bind _structout (setmembers `/Game/Quest/F_QuestInfo` :`StructRef` _value :`IsActive` true))
    (`BlueprintMapLibrary.Map_Add` (`self.QuestDatabase`) _currentid _structout)
    (`KismetArrayLibrary.Array_AddUnique` (`self.ActiveQuests`) _currentid)
    (set `self.IsPlayerInQuest` true)
    (`self.QuestActivatedWithID` (`self.CurrentID`))
    (else
      (`KismetSystemLibrary.PrintString` (`KismetStringLibrary.Concat_StrStr` "Could not activate quest with ID: " (`KismetStringLibrary.Conv_NameToString` (`BlueprintGameplayTagLibrary.GetTagName` ID)))))))

(fn `GetQuestInfoWithID`
  (params (ID :type "GameplayTag Structure (by ref)"))
  (returns (Value :type "/Game/Quest/F_QuestInfo Structure"))
  (return (`BlueprintMapLibrary.Map_Find` (`self.QuestDatabase`) ID)))