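; BP_Smoke is a smoke hazard volume that drains the player character's breath.
; On BeginPlay it caches the player as BP_RPGCharacter and sets its breath drain and fill rates.
; Box overlaps toggle the character's BreathDraining flag without checking which actor overlapped.
; Each smoke actor's Tick drains or refills breath from that flag and updates the HUD breath text.
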(event `self.ReceiveBeginPlay`
  (bind _asbp_rpgcharacter (cast `/Game/Blueprints/BP_RPGCharacter` (`GameplayStatics.GetPlayerCharacter` 0)))
  (bind _output_get (set `self.Character` _asbp_rpgcharacter))
  (set `RPGCharacter.BreathDrainRate` (`self.BreathDrainRate`) _output_get)
  (set `RPGCharacter.BreathFillRate` 15.0 _output_get))

(event `self.ReceiveTick`
  (params (DeltaSeconds :type "Float (single-precision)"))
  (bind _character (`self.Character`))
  (bind _character_2 (`self.Character`))
  (bind _returnvalue (`KismetMathLibrary.FFloor` (`RPGCharacter.Breath` _character_2)))
  (if (`RPGCharacter.BreathDraining` _character)
    (`RPGCharacter.ChangeBreath` _character DeltaSeconds true)
    (else
      (`RPGCharacter.ChangeBreath` _character DeltaSeconds false)))
  (`/Game/UI/UMG_HUD_Stats.SetBreathText` (`/Game/Blueprints/BP_RPGCharacter.HUDStats` _character_2) (`KismetTextLibrary.Conv_DoubleToText` (`KismetMathLibrary.Conv_IntToDouble` _returnvalue) "HalfToEven") (>= _returnvalue 100)))

(event `self.BoxCollision.OnComponentBeginOverlap`
  (params (OverlappedComponent :type "PrimitiveComponent Object Reference") (OtherActor :type "Actor Object Reference") (OtherComp :type "PrimitiveComponent Object Reference") (OtherBodyIndex :type Integer) (bFromSweep :type Boolean) (SweepResult :type "HitResult Structure (by ref)"))
  (set `RPGCharacter.BreathDraining` true (`self.Character`)))

(event `self.BoxCollision.OnComponentEndOverlap`
  (params (OverlappedComponent :type "PrimitiveComponent Object Reference") (OtherActor :type "Actor Object Reference") (OtherComp :type "PrimitiveComponent Object Reference") (OtherBodyIndex :type Integer))
  (set `RPGCharacter.BreathDraining` false (`self.Character`)))

(fn `UserConstructionScript`)