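; Baby deer quest actor that travels along a referenced path's spline.
; On BeginPlay it starts moving if ActivelyRunning is set, through the MoveBabyDeer event.
; A timeline with play rate scaled by Duration lerps distance over the spline length, setting world location and local-space spline rotation.
; The construction script passes ThisQuestID to its QuestComponent.
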(event `self.ReceiveBeginPlay`
  (if (`self.ActivelyRunning`)
    (`self.MoveBabyDeer`)))

(event `MoveBabyDeer`
  (bind _pathspline (`/Game/Blueprints/BP_BabyDeerPath.PathSpline` (`self.Path`)))
  (`TimelineComponent.SetPlayRate` (`self.BabyDeerMover`) (/ 1.0 (`self.Duration`)))
  (bind (_direction _alpha) (`Timeline|BabyDeerMover`)
    (:`Update`
      (bind _returnvalue (`KismetMathLibrary.Lerp` 0.0 (`SplineComponent.GetSplineLength` _pathspline) _alpha))
      (`self.K2_SetActorLocationAndRotation` (`SplineComponent.GetLocationAtDistanceAlongSpline` _pathspline _returnvalue "World") (`SplineComponent.GetRotationAtDistanceAlongSpline` _pathspline _returnvalue "Local")))))

(fn `UserConstructionScript`
  (set `/Game/Quest/QuestComponent.QuestID` (`self.ThisQuestID`) (`self.QuestComponent`)))