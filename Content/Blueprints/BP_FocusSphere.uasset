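; BP_FocusSphere is a collision sphere actor that highlights actors carrying a FocusComponent while they are inside its radius.
; Begin and end overlap events look up the FocusComponent on the other actor and switch its highlight on or off.
; Custom events resize the sphere with overlap updates and toggle it between query-only and no collision to enable or disable focusing.
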(event `SetFocusSphereSize`
  (params (InSphereRadius :type "Float (double-precision)"))
  (`SphereComponent.SetSphereRadius` (`self.SphereCollision`) InSphereRadius true))

(event `FocusOn`
  (params (On :type Boolean :default true))
  (`PrimitiveComponent.SetCollisionEnabled` (`self.SphereCollision`) (select `bool` On :`false` "NoCollision" :`true` "QueryOnly" :!type "ECollisionEnabled Enum")))

(event `self.SphereCollision.OnComponentBeginOverlap`
  (params (OverlappedComponent :type "PrimitiveComponent Object Reference") (OtherActor :type "Actor Object Reference") (OtherComp :type "PrimitiveComponent Object Reference") (OtherBodyIndex :type Integer) (bFromSweep :type Boolean) (SweepResult :type "HitResult Structure (by ref)"))
  (bind _returnvalue (`self.GetComponentByClass` OtherActor "/Game/Blueprints/FocusComponent.FocusComponent_C"))
  (`/Engine/EditorBlueprintResources/StandardMacros.IsValid` _returnvalue
    (:`Is Valid`
      (`/Game/Blueprints/FocusComponent.FocusHighlightOn` _returnvalue))))

(event `self.SphereCollision.OnComponentEndOverlap`
  (params (OverlappedComponent :type "PrimitiveComponent Object Reference") (OtherActor :type "Actor Object Reference") (OtherComp :type "PrimitiveComponent Object Reference") (OtherBodyIndex :type Integer))
  (bind _returnvalue (`self.GetComponentByClass` OtherActor "/Game/Blueprints/FocusComponent.FocusComponent_C"))
  (`/Engine/EditorBlueprintResources/StandardMacros.IsValid` _returnvalue
    (:`Is Valid`
      (`/Game/Blueprints/FocusComponent.FocushighlightOff` _returnvalue))))

(fn `UserConstructionScript`)