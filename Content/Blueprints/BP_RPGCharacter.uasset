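; Player deer character for an RPG, handling input, camera zoom, jumping, HUD, perk tree and quest log widgets.
; Each tick it highlights the registered interactable best aligned with its facing via 2D dot product and refreshes stamina text.
; AbilitiesComponent gates and tunes Dash, Rest and Focus, while Happiness drives levels and perk points.
; Also adds inventory pickups, displays active quests from a data table and quick-saves location and progression to one slot.
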(event `self.ReceiveBeginPlay`
  (`|ExecutionSequence`
    (:`then_0`
      (`|ExecutionSequence`
        (:`then_0`
          (bind _output_get (set `self.DefaultCameraBoomLength` (`SpringArmComponent.TargetArmLength` (`self.CameraBoom`))))
          (set `self.CurrentBoomLength` _output_get))
        (:`then_1`
          (set `self.DefaultFollowCameraLoc` (`SceneComponent.RelativeLocation` (`self.FollowCamera`))))
        (:`then_2`
          (`ActorComponent.Deactivate` (`self.ChargeParticles`)) ; Deactivates any particle effects on the deer
        )
        (:`then_3`
          (`KismetSystemLibrary.Delay` 1.0) ; Displays Location text
          (bind _returnvalue (`|CreateWidget` "/Game/UI/UMG_LocationText.UMG_LocationText_C"))
          (`UserWidget.AddToViewport` _returnvalue 0)
          (`KismetSystemLibrary.Delay` 5.0)
          (`Widget.RemoveFromParent` _returnvalue) ; Should remove it, probably just hide it \nbecause i want to show different locations
        )
        (:`then_4`
          (set `self.DefaultStaminaFillRate` (`self.StaminaFillRate`)))))
    (:`then_1`
      (`|ExecutionSequence`
        (:`then_0`
          (bind _returnvalue_2 (`|CreateWidget` "/Game/UI/UMG_HUD_Stats.UMG_HUD_Stats_C"))
          (bind _output_get_2 (set `self.HUDStats` _returnvalue_2))
          (`UserWidget.AddToViewport` _output_get_2 0))
        (:`then_1`
          (bind _returnvalue_3 (`|CreateWidget` "/Game/UI/UMG_HUD_ActiveQuests.UMG_HUD_ActiveQuests_C"))
          (bind _output_get_3 (set `self.HUDActiveQuests` _returnvalue_3))
          (`UserWidget.AddToViewport` _output_get_3 0))
        (:`then_2`
          (bind _returnvalue_4 (`|CreateWidget` "/Game/UI/UMG_QuestLog.UMG_QuestLog_C"))
          (bind _output_get_4 (set `self.UMGQuestLog` _returnvalue_4))
          (`UserWidget.AddToViewport` _output_get_4 0)
          (`Widget.SetVisibility` _output_get_4 "Hidden"))
        (:`then_3`
          (bind _returnvalue_5 (`|CreateWidget` "/Game/UI/UMG_PerkTree.UMG_PerkTree_C"))
          (bind _output_get_5 (set `self.UMGPerkTree` _returnvalue_5))
          (`UserWidget.AddToViewport` _output_get_5 1)
          (`Widget.SetVisibility` _output_get_5 "Hidden")
          (`self.HappinessChanged`))
        (:`then_4`
          (bind _returnvalue_6 (`|CreateWidget` "/Game/UI/UMG_HUD_Dialogue.UMG_HUD_Dialogue_C"))
          (bind _output_get_6 (set `self.HUDDialogue` _returnvalue_6))
          (`UserWidget.AddToViewport` _output_get_6 0)
          (`Widget.SetVisibility` _output_get_6 "Visible"))
        (:`then_5`
          (bind _returnvalue_7 (`|CreateWidget` "/Game/UI/UMG_HUD_Keybindings.UMG_HUD_Keybindings_C"))
          (bind _output_get_7 (set `self.HUDKeybinds` _returnvalue_7))
          (`UserWidget.AddToViewport` _output_get_7 0))))
    (:`then_2`
      (set `self.HappinessRequirementPerLevel` (`self.HappinessRequirementPerLevel`)))
    (:`then_3`
      (bind _asbp_rpggame_instance (cast `/Game/Blueprints/BP_RPGGameInstance` (`GameplayStatics.GetGameInstance`)))
      (`|ExecutionSequence`
        (:`then_0`
          (add `/Game/Blueprints/BP_RPGGameInstance.QuestActivated` _asbp_rpggame_instance (delegate `QuestActivated`)))
        (:`then_1`
          (add `/Game/Blueprints/BP_RPGGameInstance.QuestCompleted` _asbp_rpggame_instance (delegate `QuestCompleted`)))
        (:`then_2`
          (add `/Game/Blueprints/BP_RPGGameInstance.QuestUnlocked` _asbp_rpggame_instance (delegate `QuestUnlocked`)))))))

(event `QuestActivated`
  (params (ID :type "GameplayTag Structure (by ref)"))
  (`KismetSystemLibrary.PrintString` (`KismetStringLibrary.Concat_StrStr` "Char Completed " (`KismetStringLibrary.Conv_NameToString` (`BlueprintGameplayTagLibrary.GetTagName` ID)))))

(event `QuestCompleted`
  (params (ID :type "GameplayTag Structure (by ref)"))
  (`KismetSystemLibrary.PrintString` (`KismetStringLibrary.Concat_StrStr` "Char Unlocked " (`KismetStringLibrary.Conv_NameToString` (`BlueprintGameplayTagLibrary.GetTagName` ID)))))

(event `QuestUnlocked`
  (params (ID :type "GameplayTag Structure (by ref)"))
  (`KismetSystemLibrary.PrintString` (`KismetStringLibrary.Concat_StrStr` "Char Activated " (`KismetStringLibrary.Conv_NameToString` (`BlueprintGameplayTagLibrary.GetTagName` ID)))))

(event `self.ReceiveTick`
  (params (DeltaSeconds :type "Float (single-precision)"))
  (`|ExecutionSequence`
    (:`then_0`
      (`self.CheckBestInteractable`))
    (:`then_1`
      (`/Game/UI/UMG_HUD_Stats.SetStaminaText` (`self.HUDStats`) (`KismetTextLibrary.Conv_IntToText` (`KismetMathLibrary.FFloor` (`self.Stamina`)))) ; this is hot garbage
    )))

(event `LevelUpCheck`
  (bind _level (`self.level`))
  (bind _level_2 (`self.level`))
  (bind _umgperktree (`self.UMGPerkTree`))
  (if (>= (`self.Happiness`) (`|GetArrayItem` (`self.HappinessRequirementPerLevel`) _level_2))
    (set `self.Happiness` (- (`self.Happiness`) (`|GetArrayItem` (`self.HappinessRequirementPerLevel`) (`self.level`))))
    (`/Engine/EditorBlueprintResources/StandardMacros.IncrementInt` (`self.level`)
      (:`  `
        (`Widget.SetIsEnabled` (`/Game/UI/UMG_PerkTree.Button_Stamina` _umgperktree) true)
        (`Widget.SetIsEnabled` (`/Game/UI/UMG_PerkTree.Button_Grazer` _umgperktree) true))))
  (`/Game/UI/UMG_HUD_Stats.SetLevelText` (`self.HUDStats`) (`KismetTextLibrary.Conv_IntToText` (+ _level_2 1)))
  (`/Game/UI/UMG_HUD_Stats.SetHappinessText` (`self.HUDStats`) (`self.Happiness`) (`|GetArrayItem` (`self.HappinessRequirementPerLevel`) _level))
  (`/Game/UI/UMG_PerkTree.SetPointsAvailableText` (`self.UMGPerkTree`) _level)
  (set `self.PerkPoints` _level))

(event `self.HappinessChanged`
  (`self.LevelUpCheck`))

(event `/Game/Interactables/BPI_Interactor.PickUp`
  (params (ItemInfo :type "/Game/Interactables/F_ItemInfo Structure"))
  (if (< (`KismetArrayLibrary.Array_Length` (`self.Inventory`)) (`self.InventorySize`))
    (`KismetArrayLibrary.Array_AddUnique` (`self.Inventory`) ItemInfo)
    (`/Game/Interactables/BP_Interactable_Base.InventoryFeedback` (`self.HighlightedInteractable`) ItemInfo)))

(event `Active Quest Changed`
  (params (`Active Quest` :type Name))
  (bind _returnvalue (`|GetDataTableRow` "/Game/Quest/DT_QuestInfo.DT_QuestInfo" `Active Quest`)
    (:`then`
      (bind _returnvalue_2 (`|CreateWidget` "/Game/UI/UMG_HUD_ActiveQuest_Info.UMG_HUD_ActiveQuest_Info_C"))
      (bind _output_get (set `self.HUDActiveQuests_Info` _returnvalue_2))
      (`/Game/UI/UMG_HUD_ActiveQuest_Info.SetActiveQuestText` _output_get (`.QuestName_6_115CA9A44588666EA8EB0995839D3715` (break `/Game/Quest/F_QuestInfo` _returnvalue)) (`.QuestObjective_21_FAB5BAFE474D64AF3049DF9C990EEDED` (break `/Game/Quest/F_QuestInfo` _returnvalue)))
      (`/Game/UI/UMG_HUD_ActiveQuests.AddQuestToScreen` (`self.HUDActiveQuests`) _output_get))))

(event `self.OnJumped`
  (`parent.OnJumped`)
  (set `CharacterMovementComponent.bOrientRotationToMovement` false (`self.CharacterMovement`))
  (`self.DisableInput` null)
  (set `self.AllowJump` false)
  (set `self.AllowDash` false))

(event `self.OnLanded`
  (params (Hit :type "HitResult Structure (by ref)"))
  (`parent.OnLanded` Hit)
  (`self.EnableInput` null)
  (set `CharacterMovementComponent.bOrientRotationToMovement` true (`self.CharacterMovement`))
  (`KismetSystemLibrary.Delay` (`/Game/Blueprints/AbilitiesComponent.JumpCooldown` (`self.AbilitiesComponent`)))
  (set `self.AllowJump` true)
  (set `self.AllowDash` true))

(event `self.Die`
  (`KismetSystemLibrary.PrintString` "You died"))

(event `InputAction|ZoomIn`
  (params (Key :type "Key Structure"))
  (bind _currentboomlength (`self.CurrentBoomLength`))
  (:`Pressed`
    (if (>= _currentboomlength (`self.MaxZoomIn`))
      (bind _output_get (set `self.CurrentBoomLength` (- _currentboomlength (`self.IncDecZoom`))))
      (set `SpringArmComponent.TargetArmLength` _output_get (`self.CameraBoom`) :!label _label)
      (`SceneComponent.K2_SetRelativeLocation` (`self.FollowCamera`) (`KismetMathLibrary.VLerp` (`self.DefaultFollowCameraLoc`) (0.0 0.0 0.0) (`KismetMathLibrary.MapRangeClamped` (`self.CurrentBoomLength`) (`self.DefaultCameraBoomLength`) (`self.MaxZoomIn`) 0.0 1.0)) false false))))

(event `InputAction|ZoomOut`
  (params (Key :type "Key Structure"))
  (bind _currentboomlength (`self.CurrentBoomLength`))
  (:`Pressed`
    (if (<= _currentboomlength (`self.MaxZoomOut`))
      (set `self.CurrentBoomLength` (+ (`self.IncDecZoom`) _currentboomlength))
      (goto _label))))

(event `/Game/Interactables/BPI_Interactor.UnregisterInteractable`
  (params (Interactable :type "/Game/Interactables/BP_Interactable_Base Object Reference"))
  (`self.RemoveInteractableFromArray` Interactable))

(event `/Game/Interactables/BPI_Interactor.RegisterInteractable`
  (params (Interactable :type "/Game/Interactables/BP_Interactable_Base Object Reference"))
  (`self.AddInteractableToArray` Interactable))

(event `InputAction|Interact`
  (params (Key :type "Key Structure"))
  (bind _highlightedinteractable (`self.HighlightedInteractable`))
  (:`Pressed`
    (`/Engine/EditorBlueprintResources/StandardMacros.IsValid` _highlightedinteractable
      (:`Is Valid`
        (message `/Game/Interactables/BPI_Interactor.Interaction` _highlightedinteractable self)))))

(event `self.CharacterMoved`
  (if (`/Game/Blueprints/AbilitiesComponent.RestUnlocked` (`self.AbilitiesComponent`))
    (set `self.StaminaFillRate` (`self.DefaultStaminaFillRate`) :!label _label_2)
    (if (and (`self.IsResting`) (`self.RestAvailable`))
      (set `self.RestAvailable` false)
      (set `self.IsResting` false)
      (`KismetSystemLibrary.Delay` 0.9)
      (`CharacterMovementComponent.SetMovementMode` (`self.CharacterMovement`) "MOVE_Walking" 0)
      (set `self.RestAvailable` true :!label _label_3))))

(event `InputAction|Rest`
  (params (Key :type "Key Structure"))
  (:`Pressed`
    (if (`/Game/Blueprints/AbilitiesComponent.RestUnlocked` (`self.AbilitiesComponent`))
      (if (and (<= (`KismetMathLibrary.VSize` (`self.GetVelocity`)) (`self.RestingSpeedThreshold`)) (not (`self.IsResting`)) (`self.RestAvailable`))
        (set `self.RestAvailable` false)
        (set `self.IsResting` true)
        (`CharacterMovementComponent.SetMovementMode` (`self.CharacterMovement`) "MOVE_None" 0)
        (`self.DisableInput` null)
        (`KismetSystemLibrary.Delay` 1.0)
        (`self.RestoreStamina`)
        (`self.EnableInput` null)
        (goto _label_3)
        (else
          (goto _label_2))))))

(event `DashCDReset`
  (set `/Game/Blueprints/AbilitiesComponent.DashOnCD` false (`self.AbilitiesComponent`)))

(event `Key|Zero`
  (params (Key :type "Key Structure"))
  (bind _abilitiescomponent (`self.AbilitiesComponent`))
  (bind _abilitiescomponent_2 (`self.AbilitiesComponent`))
  (:`Pressed`
    (if (and (`/Game/Blueprints/AbilitiesComponent.DashUnlocked` _abilitiescomponent_2) (>= (`self.Stamina`) (`KismetMathLibrary.Abs` (`/Game/Blueprints/AbilitiesComponent.DashCost` _abilitiescomponent_2))) (<= (`/Game/Blueprints/AbilitiesComponent.RequiredRunningVelocity` _abilitiescomponent_2) (`KismetMathLibrary.VSize` (`self.GetVelocity`))) (`self.AllowDash`) (not (`/Game/Blueprints/AbilitiesComponent.DashOnCD` (`self.AbilitiesComponent`)))) :!label _label_4
      (set `/Game/Blueprints/AbilitiesComponent.DashOnCD` true (`self.AbilitiesComponent`))
      (set `self.IsDashingAnimation` true)
      (`self.AddStamina` (* (`/Game/Blueprints/AbilitiesComponent.DashCost` _abilitiescomponent) -1.0))
      (`ActorComponent.Activate` (`self.ChargeParticles`) false)
      (set `CharacterMovementComponent.bOrientRotationToMovement` false (`self.CharacterMovement`))
      (`self.LaunchCharacter` (* (`self.GetVelocity`) (`/Game/Blueprints/AbilitiesComponent.DashMultiplier` _abilitiescomponent)))
      (`self.DisableInput` null)
      (`|ExecutionSequence`
        (:`then_0`
          (`KismetSystemLibrary.Delay` 0.2)
          (set `MovementComponent.Velocity` (* (`self.GetVelocity`) (`/Game/Blueprints/AbilitiesComponent.DashMultiplier` _abilitiescomponent)) (`self.CharacterMovement`)) ; Right after dash is over, set velocity \nso that you dont slow down after dash
          (`ActorComponent.Deactivate` (`self.ChargeParticles`)))
        (:`then_1`
          (`KismetSystemLibrary.Delay` 0.4)
          (`self.EnableInput` null)
          (set `self.IsDashingAnimation` false)
          (`KismetSystemLibrary.K2_SetTimerDelegate` (delegate `DashCDReset`) (`/Game/Blueprints/AbilitiesComponent.DashCooldown` (`self.AbilitiesComponent`))))))))

(event `Key|F`
  (params (Key :type "Key Structure"))
  (:`Pressed`
    (goto _label_4)))

(event `Key|L`
  (params (Key :type "Key Structure"))
  (bind _umgquestlog (`self.UMGQuestLog`))
  (:`Pressed`
    (`/Engine/EditorBlueprintResources/StandardMacros.FlipFlop`
      (:`A`
        (`CharacterMovementComponent.SetMovementMode` (`self.CharacterMovement`) "MOVE_None" 0)
        (`Widget.SetVisibility` _umgquestlog "Visible"))
      (:`B`
        (`CharacterMovementComponent.SetMovementMode` (`self.CharacterMovement`) "MOVE_Walking" 0)
        (`Widget.SetVisibility` _umgquestlog "Hidden")))))

(event `Key|T`
  (params (Key :type "Key Structure"))
  (bind _returnvalue (`GameplayStatics.GetPlayerController` 0))
  (bind _umgperktree (`self.UMGPerkTree`))
  (:`Pressed`
    (`/Engine/EditorBlueprintResources/StandardMacros.FlipFlop`
      (:`A`
        (`CharacterMovementComponent.SetMovementMode` (`self.CharacterMovement`) "MOVE_None" 0)
        (`Widget.SetVisibility` _umgperktree "Visible")
        (`WidgetBlueprintLibrary.SetInputMode_GameAndUIEx` _returnvalue null "DoNotLock" false)
        (set `PlayerController.bShowMouseCursor` true _returnvalue))
      (:`B`
        (`CharacterMovementComponent.SetMovementMode` (`self.CharacterMovement`) "MOVE_Walking" 0)
        (`Widget.SetVisibility` _umgperktree "Hidden")
        (`WidgetBlueprintLibrary.SetInputMode_GameOnly` _returnvalue)
        (set `PlayerController.bShowMouseCursor` false _returnvalue)))))

(event `Key|H`
  (params (Key :type "Key Structure"))
  (:`Pressed`
    (bind _returnvalue (`GameplayStatics.CreateSaveGameObject` "/Game/Blueprints/BP_Save.BP_Save_C"))
    (bind _output_get (set `self.Save` _returnvalue))
    (bind _output_get_2 (set `self.PlayerLocation` (`self.K2_GetActorLocation`)))
    (set `/Game/Blueprints/BP_Save.PlayerLocation_Save` _output_get_2 _output_get)
    (set `/Game/Blueprints/BP_Save.PlayerHappiness_Save` (`self.Happiness`) _output_get)
    (set `/Game/Blueprints/BP_Save.PlayerLevel_Save` (`self.level`) _output_get)
    (set `/Game/Blueprints/BP_Save.PlayerPerkPoints_Save` (`self.PerkPoints`) _output_get)
    (`GameplayStatics.SaveGameToSlot` _output_get "test")
    (`KismetSystemLibrary.PrintString` "GAME HAS BEEN SAVED" true true (struct :`R` 0.024615 :`G` 1.0 :`A` 1.0))))

(event `Key|J`
  (params (Key :type "Key Structure"))
  (:`Pressed`
    (bind _returnvalue (`GameplayStatics.DoesSaveGameExist` "test"))
    (if _returnvalue
      (bind _returnvalue_2 (`GameplayStatics.LoadGameFromSlot` "test"))
      (bind _asbp_save (cast `/Game/Blueprints/BP_Save` _returnvalue_2))
      (bind _output_get (set `self.PlayerLocation` (`/Game/Blueprints/BP_Save.PlayerLocation_Save` _asbp_save)))
      (`self.K2_SetActorLocation` _output_get)
      (set `self.Happiness` (`/Game/Blueprints/BP_Save.PlayerHappiness_Save` _asbp_save))
      (set `self.level` (`/Game/Blueprints/BP_Save.PlayerLevel_Save` _asbp_save))
      (set `self.PerkPoints` (`/Game/Blueprints/BP_Save.PlayerPerkPoints_Save` _asbp_save))
      (set `self.HUDActiveQuests` (`/Game/Blueprints/BP_Save.ActiveQuest_Widget_Save` _asbp_save))
      (`self.HappinessChanged`)
      (`KismetSystemLibrary.PrintString` "LOAD SUCCESSFUL" true true (struct :`R` 0.155521 :`G` 1.0 :`A` 1.0))
      (else
        (`KismetSystemLibrary.PrintString` "NO DATA TO LOAD")))))

(event `Key|Q`
  (params (Key :type "Key Structure"))
  (bind _abilitiescomponent (`self.AbilitiesComponent`))
  (bind _focuscost (`/Game/Blueprints/AbilitiesComponent.FocusCost` _abilitiescomponent))
  (:`Pressed`
    (if (and (`/Game/Blueprints/AbilitiesComponent.FocusUnlocked` _abilitiescomponent) (`self.CanAffordStaminaCost` _focuscost) (not (`/Game/Blueprints/AbilitiesComponent.FocusOnCD` (`self.AbilitiesComponent`))))
      (set `/Game/Blueprints/AbilitiesComponent.FocusOnCD` true (`self.AbilitiesComponent`))
      (`self.AddStamina` (* _focuscost -1.0))
      (bind _asbp_focus_sphere (cast `/Game/Blueprints/BP_FocusSphere` (`ChildActorComponent.ChildActor` (`self.FocusSphereChildActor`))))
      (`/Game/Blueprints/BP_FocusSphere.FocusOn` _asbp_focus_sphere true)
      (`|ExecutionSequence`
        (:`then_0`
          (`KismetSystemLibrary.Delay` (`/Game/Blueprints/AbilitiesComponent.FocusDuration` (`self.AbilitiesComponent`)))
          (`/Game/Blueprints/BP_FocusSphere.FocusOn` _asbp_focus_sphere false))
        (:`then_1`
          (`KismetSystemLibrary.Delay` (`/Game/Blueprints/AbilitiesComponent.FocusCooldown` (`self.AbilitiesComponent`)))
          (set `/Game/Blueprints/AbilitiesComponent.FocusOnCD` false (`self.AbilitiesComponent`)))))))

(event `Key|One`
  (params (Key :type "Key Structure"))
  (:`Pressed`
    (`self.AddStamina` 100.0)))

(event `Key|Two`
  (params (Key :type "Key Structure"))
  (:`Pressed`
    (`self.AddHappiness` 50 true)))

(event `self.FocusCollisionSphere.OnComponentBeginOverlap`
  (params (OverlappedComponent :type "PrimitiveComponent Object Reference") (OtherActor :type "Actor Object Reference") (OtherComp :type "PrimitiveComponent Object Reference") (OtherBodyIndex :type Integer) (bFromSweep :type Boolean) (SweepResult :type "HitResult Structure (by ref)"))
  (bind _returnvalue (`self.GetComponentByClass` OtherActor "/Game/Blueprints/FocusComponent.FocusComponent_C"))
  (`/Engine/EditorBlueprintResources/StandardMacros.IsValid` _returnvalue
    (:`Is Valid`
      (`/Game/Blueprints/FocusComponent.FocusHighlightOn` _returnvalue))))

(event `self.FocusCollisionSphere.OnComponentEndOverlap`
  (params (OverlappedComponent :type "PrimitiveComponent Object Reference") (OtherActor :type "Actor Object Reference") (OtherComp :type "PrimitiveComponent Object Reference") (OtherBodyIndex :type Integer))
  (bind _returnvalue (`self.GetComponentByClass` OtherActor "/Game/Blueprints/FocusComponent.FocusComponent_C"))
  (`/Engine/EditorBlueprintResources/StandardMacros.IsValid` _returnvalue
    (:`Is Valid`
      (`/Game/Blueprints/FocusComponent.FocushighlightOff` _returnvalue))))

(fn `AddInteractableToArray`
  (params (Interactable :type "/Game/Interactables/BP_Interactable_Base Object Reference"))
  (`KismetArrayLibrary.Array_AddUnique` (`self.Interactables`) Interactable))

(fn `CanJumpInternal`
  (returns (ReturnValue :type Boolean))
  (return (`self.AllowJump`)))

(fn `CheckBestInteractable`
  (if (> (`KismetArrayLibrary.Array_Length` (`self.Interactables`)) 0)
    (`self.GetBestInteractable`)
    (else
      (`self.SetBestInteractable` null))))

(fn `Dash`)

(fn `GetBestInteractable`
  (locals (InteractableVariables :type "/Game/Interactables/F_InteractableDot Structure"))
  (bind _interactablevariables_dot (break `/Game/Interactables/F_InteractableDot` (`local.InteractableVariables`)))
  (bind (_interactablevariables_dot_2 _interactablevariables_interactable) (break `/Game/Interactables/F_InteractableDot` (`local.InteractableVariables`)))
  (bind _capsulecomponent (`self.CapsuleComponent`))
  (bind (_returnvalue_x _returnvalue_y) (`KismetMathLibrary.BreakVector` (`SceneComponent.K2_GetComponentLocation` _capsulecomponent)))
  (bind (_returnvalue_x_2 _returnvalue_y_2) (`KismetMathLibrary.BreakVector` (`SceneComponent.GetForwardVector` _capsulecomponent)))
  (set `local.InteractableVariables` (make `/Game/Interactables/F_InteractableDot` -1.0))
  (for _array_element (`self.Interactables`)
    (bind (_returnvalue_x_3 _returnvalue_y_3) (`KismetMathLibrary.BreakVector` (`SceneComponent.K2_GetComponentLocation` (`/Game/Interactables/BP_Interactable_Base.InteractionPoint` _array_element))))
    (bind _returnvalue (`KismetMathLibrary.Dot_VectorVector` (`KismetMathLibrary.Normal` (- (`KismetMathLibrary.MakeVector` _returnvalue_x_3 _returnvalue_y_3) (`KismetMathLibrary.MakeVector` _returnvalue_x _returnvalue_y))) (`KismetMathLibrary.MakeVector` _returnvalue_x_2 _returnvalue_y_2)))
    (if (and (> _returnvalue (`self.DotAngle`)) (> _returnvalue _interactablevariables_dot))
      (set `local.InteractableVariables` (make `/Game/Interactables/F_InteractableDot` _returnvalue _array_element))))
  (`/Engine/EditorBlueprintResources/StandardMacros.IsValid` _interactablevariables_interactable
    (:`Is Valid`
      (`self.SetBestInteractable` _interactablevariables_interactable))
    (:`Is Not Valid`
      (`self.SetBestInteractable` null))))

(fn `RemoveInteractableFromArray`
  (params (Interactable :type "/Game/Interactables/BP_Interactable_Base Object Reference"))
  (`KismetArrayLibrary.Array_RemoveItem` (`self.Interactables`) Interactable))

(fn `RestoreStamina`
  (set `self.StaminaFillRate` (* (`self.StaminaFillMultiplier`) (`self.DefaultStaminaFillRate`))))

(fn `SetBestInteractable`
  (params (Interactable :type "/Game/Interactables/BP_Interactable_Base Object Reference"))
  (`/Engine/EditorBlueprintResources/StandardMacros.IsValid` Interactable
    (:`Is Valid`
      (if (!= Interactable (`self.HighlightedInteractable`))
        (bind _highlightedinteractable (`self.HighlightedInteractable`)
          (:`then`
            (`/Game/Interactables/BP_Interactable_Base.SetFeedback` _highlightedinteractable false))
          (:`else`
            _))
        (bind _output_get (set `self.HighlightedInteractable` Interactable))
        (`/Game/Interactables/BP_Interactable_Base.SetFeedback` _output_get true)))
    (:`Is Not Valid`
      (bind _highlightedinteractable_2 (`self.HighlightedInteractable`)
        (:`then`
          (`/Game/Interactables/BP_Interactable_Base.SetFeedback` _highlightedinteractable_2 false)
          (set `self.HighlightedInteractable` null))
        (:`else`)))))

(fn `UserConstructionScript`
  (set `/Game/Blueprints/AbilitiesComponent.Character` self (`self.AbilitiesComponent`)))