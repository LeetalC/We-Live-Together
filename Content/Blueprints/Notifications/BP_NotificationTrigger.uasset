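; Trigger actor that shows a one-time tutorial notification popup when something overlaps its collider.
; On BeginPlay it caches the player's BP_RPGCharacter to reach the HUD widget.
; Any overlap, with no actor filter, interrupts the notification manager's queue, then looks up RowNameNotification in DT_Notification.
; If the row exists, its text goes to the tutorial popup and the trigger destroys itself.
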(event `self.ReceiveBeginPlay`
  (`|ExecutionSequence`
    (:`then_0`
      (bind _asbp_rpgcharacter (cast `/Game/Blueprints/BP_RPGCharacter` (`GameplayStatics.GetPlayerCharacter` 0)))
      (set `self.Character` _asbp_rpgcharacter))))

(event `self.TriggerDialogueCollider.OnComponentBeginOverlap`
  (params (OverlappedComponent :type "PrimitiveComponent Object Reference") (OtherActor :type "Actor Object Reference") (OtherComp :type "PrimitiveComponent Object Reference") (OtherBodyIndex :type Integer) (bFromSweep :type Boolean) (SweepResult :type "HitResult Structure (by ref)"))
  (`self.NotificationTriggered`))

(event `NotificationTriggered`
  (`/Game/UI/Notifications/UMG_NotificationManager.InterruptQueue` (`/Game/UI/UMG_MainHUD.UMG_NotificationManager` (`/Game/Blueprints/BP_RPGCharacter.HUDWidget` (`self.Character`))))
  (bind _returnvalue (`|GetDataTableRow` "/Game/Blueprints/Notifications/DT_Notification.DT_Notification" (`self.RowName_Notification`))
    (:`then`
      (`/Game/UI/Notifications/UMG_TutorialPopup.ActivateNotificationPopup` (`/Game/UI/UMG_MainHUD.UMG_TutorialPopup` (`/Game/Blueprints/BP_RPGCharacter.HUDWidget` (`self.Character`))) (`.Text_5_6707EE2D43BB85E5B6CF51A2EE4CAEEE` (break `/Game/Blueprints/Dialogue/F_Dialogue` _returnvalue)))
      (`self.K2_DestroyActor`))))

(fn `UserConstructionScript`)