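; BP_LocationTextTrigger is a one-shot trigger volume that announces a location name on the HUD and updates background music.
; BeginPlay caches the RPG character and game mode.
; Any overlap disables the collider and sets the game mode's BGMusic, calling MusicChanged only when AreaHasUniqueMusic is true.
; It then plays the location text through the character's HUD widget and destroys itself.
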(event `self.ReceiveBeginPlay`
  (`|ExecutionSequence`
    (:`then_0`
      (bind _asbp_rpgcharacter (cast `/Game/Blueprints/BP_RPGCharacter` (`GameplayStatics.GetPlayerCharacter` 0)))
      (set `self.Character` _asbp_rpgcharacter))
    (:`then_1`
      (bind _asbp_rpggame_mode (cast `/Game/Blueprints/BP_RPGGameMode` (`GameplayStatics.GetGameMode`)))
      (set `self.GameMode` _asbp_rpggame_mode))))

(event `self.TriggerDialogueCollider.OnComponentBeginOverlap`
  (params (OverlappedComponent :type "PrimitiveComponent Object Reference") (OtherActor :type "Actor Object Reference") (OtherComp :type "PrimitiveComponent Object Reference") (OtherBodyIndex :type Integer) (bFromSweep :type Boolean) (SweepResult :type "HitResult Structure (by ref)"))
  (bind _gamemode (`self.GameMode`))
  (`|ExecutionSequence`
    (:`then_0`
      (`PrimitiveComponent.SetCollisionEnabled` (`self.TriggerDialogueCollider`) "NoCollision")
      (set `/Game/Blueprints/BP_RPGGameMode.BGMusic` (`self.BGMusic`) _gamemode)
      (if (`self.AreaHasUniqueMusic`)
        (`/Game/Blueprints/BP_RPGGameMode.MusicChanged` _gamemode)))
    (:`then_1`
      (`/Game/UI/Notifications/UMG_LocationText.PlayLocationText` (`/Game/UI/UMG_MainHUD.UMG_LocationText` (`/Game/Blueprints/BP_RPGCharacter.HUDWidget` (`self.Character`))) (`self.Location`))
      (`self.K2_DestroyActor`))))

(fn `UserConstructionScript`)